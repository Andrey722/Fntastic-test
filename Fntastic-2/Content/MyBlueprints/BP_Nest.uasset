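; BP_Nest is a spawn point that creates turtles for what appears to be a race toward a finish line.
; SpawnTurtle spawns the turtle class at the nest's transform, begins the Sparks trail effect and sets a one-shot timer.
; It passes the turtle's controller to FinishLine, turns the turtle to face that line and returns the controller.
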(fn `SpawnTurtle`
  (returns (ReturnValue :type "TurtleController Object Reference"))
  (bind _finishline (`self.FinishLine`))
  (if (`KismetSystemLibrary.IsValidClass` (`self.TurtleClass`))
    (bind _returnvalue (`|SpawnActorFromClass` (`self.TurtleClass`) (`KismetMathLibrary.MakeTransform` (`self.K2_GetActorLocation`) (`self.K2_GetActorRotation`)) "AdjustIfPossibleButAlwaysSpawn" "OverrideRootScale" null null))
    (bind _asturtle_controller (cast `TurtleController` (`Pawn.GetController` _returnvalue)))
    (`ParticleSystemComponent.BeginTrails` (`self.Sparks`) "None" "None" "ETrailWidthMode_FromCentre" 0.0)
    (`KismetSystemLibrary.K2_SetTimerDelegate` (`|CreateDelegate` :!event `StopSpawnVisual`) 4.0)
    (`FinishTrigger.OnTurtleSpawned` _finishline _asturtle_controller)
    (`self.K2_SetActorRotation` _returnvalue (`KismetMathLibrary.FindLookAtRotation` (`self.K2_GetActorLocation`) (`self.K2_GetActorLocation` _finishline)) false)
    (return _asturtle_controller)))

(fn `UserConstructionScript`)